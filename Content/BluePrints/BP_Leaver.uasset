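; BP_Leaver is an interactable lever that toggles between on and off and drives other actors in the level.
; Interacting plays or reverses a timeline that rotates the handle between start and end rotations, with the active state set from the timeline direction when it finishes.
; It then sends that state to each linked interactable through BPI_Interactable and, only the first time, plays an assigned level sequence.
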(event `self.ReceiveBeginPlay`)

(event `Interacted`
  (bind _isactive (`self.IsActive`))
  (bind _sequenceplayer (`LevelSequenceActor.SequencePlayer` (`self.LeveSequence`)))
  ;[0.301 0.301 0.301] Animation Lever
  (if (not (`self.IsActive`))
    (bind (_direction _alpha) (`Timeline|LeverAnim` :!label _label)
      (:`Update`
        (`SceneComponent.K2_SetRelativeRotation` (`self.Leaver_Leaver`) (`KismetMathLibrary.RLerp` (`self.StartRotation`) (`self.EndRotation`) _alpha true) false false))
      (:`Finished`
        (`|ExecutionSequence`
          (:`then_0`
            (set `self.IsActive` (select `ETimelineDirection` _direction :`Forward` true)))
          (:`then_1`
            ;[0.2427 0.1562 0.2362] ActorToTriggerLoop
            (for _array_element (`self.Interactables`)
              (if (`KismetSystemLibrary.DoesImplementInterface` _array_element "/Game/BluePrints/Interfaces/BPI_Interactable.BPI_Interactable_C")
                (message `/Game/BluePrints/Interfaces/BPI_Interactable.Interact` _array_element _isactive)
                (message `/Game/BluePrints/Interfaces/BPI_Trigger.Trigger` _array_element _isactive self))))
          (:`then_2`
            ;[0.3552 0.06771 0.06771] PlayLevelSquence
            (`/Engine/EditorBlueprintResources/StandardMacros.DoOnce` false
              (:`Completed`
                (`/Engine/EditorBlueprintResources/StandardMacros.IsValid` _sequenceplayer
                  (:`Is Valid`
                    (`MovieSceneSequencePlayer.Play` _sequenceplayer)))))))))
    (else
      (goto _label :!via `Reverse`))))

(event `Interact_1_1`
  (params (NewParam :type "Actor Object Reference"))
  ;[0.301 0.301 0.301] Animation Lever
  (`self.Interacted`))

(fn `Interact`
  (params (On :type Boolean)))

(fn `UserConstructionScript`)