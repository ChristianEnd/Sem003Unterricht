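; Atmosphere audio zone for a canyon ("Schlucht") that plays ambient sound while a triggering actor is inside it.
; Overlapping Outerrim with an actor implementing BPI_AtmoTrigger plays and unpauses AtmoSchlucht; leaving pauses it, as does BeginPlay.
; A radial volume change toward Innerrim is marked TODO, with only disconnected cast, lerp and distance nodes present.
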(event `self.ReceiveTick`
  (params (DeltaSeconds :type "Float (single-precision)"))
  ;[1 1 1] TODORADIALVolumeChange
)

(event `self.Outerrim.OnComponentBeginOverlap`
  (params (OverlappedComponent :type "PrimitiveComponent Object Reference") (OtherActor :type "Actor Object Reference") (OtherComp :type "PrimitiveComponent Object Reference") (OtherBodyIndex :type Integer) (bFromSweep :type Boolean) (SweepResult :type "HitResult Structure (by ref)"))
  (bind _atmoschlucht (`self.AtmoSchlucht`))
  (if (`KismetSystemLibrary.DoesImplementInterface` OtherActor "/Game/BluePrints/Interfaces/BPI_AtmoTrigger.BPI_AtmoTrigger_C")
    (`|ExecutionSequence`
      (:`then_0`
        (`FMODAudioComponent.Play` _atmoschlucht))
      (:`then_1`
        (`FMODAudioComponent.SetPaused` _atmoschlucht false)))))

(event `self.Outerrim.OnComponentEndOverlap`
  (params (OverlappedComponent :type "PrimitiveComponent Object Reference") (OtherActor :type "Actor Object Reference") (OtherComp :type "PrimitiveComponent Object Reference") (OtherBodyIndex :type Integer))
  (if (`KismetSystemLibrary.DoesImplementInterface` OtherActor "/Game/BluePrints/Interfaces/BPI_AtmoTrigger.BPI_AtmoTrigger_C")
    (`FMODAudioComponent.SetPaused` (`self.AtmoSchlucht`) true :!label _label)))

(event `self.ReceiveBeginPlay`
  (goto _label))

(fn `UserConstructionScript`)