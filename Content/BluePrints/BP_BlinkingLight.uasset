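; BP_BlinkingLight is a spot light that blinks and switches to green when triggered on.
; BeginPlay starts the BlinkingInterval timeline, whose track interpolates intensity between zero and LightIntensity.
; Each timeline update also sets the color: a hardcoded green while On is true, otherwise NewLightColor.
; The Trigger event only stores the On flag, so the color change appears on timeline updates.
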(event `self.ReceiveBeginPlay`
  (`self.Blink`))

(event `Blink`
  (bind _spotlight (`self.SpotLight`))
  (bind (_direction _newtrack_0) (`Timeline|BlinkingInterval`)
    (:`Update`
      (`LightComponent.SetIntensity` _spotlight (`KismetMathLibrary.Lerp` 0.0 (`self.LightIntensity`) _newtrack_0))
      (if (`self.On`)
        (`LightComponent.SetLightColor` _spotlight (struct :`R` 0.008647 :`G` 1.0 :`A` 1.0) true)
        (else
          (`LightComponent.SetLightColor` _spotlight (`self.New Light Color`) true))))))

(event `/Game/BluePrints/Interfaces/BPI_Trigger.Trigger`
  (params (On :type Boolean) (Actor :type "Actor Object Reference"))
  (set `self.On` On))

(fn `UserConstructionScript`)