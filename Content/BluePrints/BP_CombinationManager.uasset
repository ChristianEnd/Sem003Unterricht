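; Combination puzzle manager that tracks which actors are switched on through its Trigger event and can activate a list of target actors.
; Trigger adds or removes the sender in CurrentCombination, then, once its length equals WantedCombination's, looks up each wanted element regardless of order.
; As written, the loop breaks on a found element despite its mistake-check label, so TriggerMessage(On) reaches interface-implementing ActorsToTrigger only when none match.
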(event `/Game/BluePrints/Interfaces/BPI_Trigger.Trigger`
  (params (On :type Boolean) (Actor :type "Actor Object Reference"))
  ;[1 1 1] RemoveTriggeredObjectFromList
  (if On
    (`KismetArrayLibrary.Array_Add` (`self.CurrentCombination`) Actor)
    (if (== (`KismetArrayLibrary.Array_Length` (`self.CurrentCombination`)) (`KismetArrayLibrary.Array_Length` (`self.WantedCombination`))) :!label _label
      (set `self.IsLoopBroken` false)
      ;[1 1 1] CheckIfCombinationIsCorrect
      (for _array_element (`self.WantedCombination`) :!label _label_2
        (if (!= (`KismetArrayLibrary.Array_Find` (`self.CurrentCombination`) _array_element) -1)
          ;[1 1 1] StopLoopIfMistakeFound
          (`self.BreakLoop`)
          (set `self.IsLoopBroken` true)))
      (if (not (`self.IsLoopBroken`))
        (`|ExecutionSequence`
          (:`then_0`
            (for _array_element_2 (`self.ActorsToTrigger`)
              (if (`KismetSystemLibrary.DoesImplementInterface` _array_element_2)
                (message `/Game/BluePrints/Interfaces/BPI_Trigger.Trigger` _array_element_2 true null)))))))
    (elif (!= (`KismetArrayLibrary.Array_Find` (`self.CurrentCombination`) Actor) -1)
      (`KismetArrayLibrary.Array_RemoveItem` (`self.CurrentCombination`) Actor)
      (goto _label))))

(event `BreakLoop`
  ;[1 1 1] CheckIfCombinationIsCorrect
  (goto _label_2 :!via `Break`))

(fn `UserConstructionScript`)