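; BP_Falling is a falling prop built from a Box and Crystal that drops when triggered.
; Its Trigger event, when switched on, enables physics on both components and destroys the actor after a short delay.
; A Box hit against any actor implementing BPI_Trigger also destroys it after a delay.
; The construction script and Boop function are empty.
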(event `self.Box.OnComponentHit`
  (params (HitComponent :type "PrimitiveComponent Object Reference") (OtherActor :type "Actor Object Reference") (OtherComp :type "PrimitiveComponent Object Reference") (NormalImpulse :type "Vector Structure") (Hit :type "HitResult Structure (by ref)"))
  ;[1 1 1] OnHitDissolve
  (if (`KismetSystemLibrary.DoesImplementInterface` OtherActor "/Game/BluePrints/Interfaces/BPI_Trigger.BPI_Trigger_C")
    (`KismetSystemLibrary.Delay` 1.0)
    (`self.K2_DestroyActor`)))

(event `/Game/BluePrints/Interfaces/BPI_Trigger.Trigger`
  (params (On :type Boolean) (Actor :type "Actor Object Reference"))
  ;[1 1 1] FallAction
  (if On
    (`PrimitiveComponent.SetSimulatePhysics` (`self.Box`) true)
    (`PrimitiveComponent.SetSimulatePhysics` (`self.Crystal`) true)
    (`KismetSystemLibrary.Delay` 1.5)
    (`self.K2_DestroyActor`)))

(fn `Boop`
  (returns (Other :type "Actor Object Reference"))
  (return null))

(fn `UserConstructionScript`)