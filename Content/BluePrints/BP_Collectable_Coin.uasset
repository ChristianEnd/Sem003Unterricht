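; Collectable coin actor that spins, bobs and adds its value to the score when collected.
; On BeginPlay it stores its origin and starts the CoinAnim timeline, which drives the mesh's rotation and vertical bounce.
; The Collect event uses a second timeline to move the coin to the Collector, then calls AddScore on GM_Basic and destroys it.
; Scale is set from that timeline's alpha only once per Collect call, outside its update.
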(event `self.ReceiveBeginPlay`
  (`self.Animate`)
  (set `self.CoinOrigin` (`self.K2_GetActorLocation`)))

(event `Animate`
  (bind (_direction _alpha _alpha__bounce) (`Timeline|CoinAnim` :!via `PlayFromStart`)
    (:`Update`
      (`SceneComponent.K2_SetWorldRotation` (`self.Münze`) (`KismetMathLibrary.RLerp` (struct) (struct :`Yaw` 360.0) _alpha) false false)
      (`SceneComponent.K2_SetRelativeLocation` (`self.Münze`) (`KismetMathLibrary.VLerp` (0.0 0.0 -10.0) (0.0 0.0 0.0) _alpha__bounce) false false))))

(event `/Game/BluePrints/Interfaces/BPI_Collectable.Collect`
  (params (Collector :type "Pawn Object Reference"))
  (`|ExecutionSequence`
    (:`then_0`
      (bind (_direction _alpha) (`Timeline|CollectCoin`)
        (:`Update`
          (`self.K2_SetActorLocation` (`KismetMathLibrary.VLerp` (`self.CoinOrigin`) (`self.K2_GetActorLocation` Collector) _alpha)))
        (:`Finished`
          (bind _asgm_basic (cast `/Game/BluePrints/GM_Basic` (`GameplayStatics.GetGameMode`)))
          (`/Game/BluePrints/GM_Basic.AddScore` _asgm_basic (`self.Value`))
          (`self.K2_DestroyActor`))))
    (:`then_1`
      (`self.SetActorScale3D` (`KismetMathLibrary.VLerp` (1.0 1.0 1.0) (0.0 0.0 0.0) _alpha)))))

(fn `UserConstructionScript`
  (`parent.UserConstructionScript`))